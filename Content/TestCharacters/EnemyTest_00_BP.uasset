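; Test enemy Blueprint with a toggleable lock-on marker, player seeking and position reporting.
; If alive at BeginPlay, a looping timer frequently writes its location to the GameInstance's TargetPosition.
; Lockon alternately shows and hides the Target component via a FlipFlop.
; SeekPlayer runs AI MoveTo toward the player controller rather than the character, and a helper returns distance to the player character.
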(event Custom|SeekPlayer
  (AI|AIMoveTo self "0, 0, 0" (Game|GetPlayerController 0) 1e+02 false))

(event EventBeginPlay
  (if (Variables|Default|GetAlive)
    (Utilities|FlowControl|DoOnce false
      (:Completed
        (Utilities|Time|SetTimerbyFunctionName 0 "SendTargetLocation" 0.05 true)))))

(event EventLockon
  (bind _target (Variables|Default|Gettarget))
  (Utilities|FlowControl|FlipFlop
    (:A
      (Development|SetHiddeninGame _target false false))
    (:B
      (Development|SetHiddeninGame _target true false))))

(fn ConstructionScript)

(fn SendTargetLocation
  (bind _asgame_instance_gi (Utilities|Casting|CastToGameInstance_GI (Game|GetGameInstance)))
  (Variables|/Game/General_Blueprints/GameInstance_GI.GameInstance_GI_C|SetTargetPosition _asgame_instance_gi (Transformation|GetActorLocation)))

(fn PlayerDistanceCheck
  (return (Transformation|GetDistanceTo (Game|GetPlayerCharacter 0))))