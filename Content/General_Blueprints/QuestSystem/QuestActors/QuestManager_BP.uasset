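; QuestManager Blueprint that adds quests to the game and tracks which one is currently selected.
; AddNewQuest rejects invalid or duplicate quest classes, spawns the quest actor, sets up its start goals and links it to a list entry in the main widget.
; A new quest is auto-selected on direct start or when it is the first one.
; SelectNewQuest disables the previous quest's name widget and activates the new quest's chosen subgoal.
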(event Custom|OnSwitch_SubQuest)

(fn ConstructionScript)

(fn SelectNewQuest
  (params (Quest :type Master%20Quest%20BP%20Object%20Reference) (SubGoal :type Sub%20Goal%20Widget%20Object%20Reference))
  (Utilities|IsValid (Variables|Default|GetCurrentQuest)
    (:Is%20Valid
      (Widget|SetIsEnabled (Variables|/Game/UI_HUD_Blueprints/Quest_Widget.Quest_Widget_C|GetQuestName (Variables|/Game/General_Blueprints/QuestSystem/QuestActors/MasterQuest_BP.MasterQuest_BP_C|GetQuestWidget (Variables|Default|GetCurrentQuest))) false)
      (Default|SelectSubGoals (Variables|/Game/General_Blueprints/QuestSystem/QuestActors/MasterQuest_BP.MasterQuest_BP_C|GetQuestWidget (Variables|Default|GetCurrentQuest))))
    (:Is%20Not%20Valid
      _))
  (bind _output_get (Variables|Default|SetCurrentQuest Quest))
  (Default|OnQuestSelected (Variables|/Game/General_Blueprints/QuestSystem/QuestActors/MasterQuest_BP.MasterQuest_BP_C|GetQuestWidget _output_get) SubGoal)
  (return))

(fn AddNewQuest
  (params (QuestClass :type Master%20Quest%20BP%20Class%20Reference) (DirectStart? :type Boolean))
  (LocalVariables|SetLocalClass QuestClass)
  (LocalVariables|SetStart? DirectStart?)
  (if (and (Utilities|IsValidClass QuestClass) (not (Utilities|Array|ContainsItem (Variables|Default|GetAllQuestClasses) QuestClass)))
    (Utilities|Array|Add (Variables|Default|GetAllQuestClasses) (LocalVariables|GetLocalClass))
    (bind _returnvalue (Game|SpawnActorfromClass (LocalVariables|GetLocalClass) (Math|Transform|MakeTransform "0, 0, 0" "0, 0, 0" "1,1,1") "AlwaysSpawn" 0 0))
    (bind _output_get (LocalVariables|SetLocalQuestActor _returnvalue))
    (Utilities|Array|Add (Variables|Default|GetQuestActors) _output_get)
    (Default|SetupStartGoals (LocalVariables|GetLocalQuestActor))
    (bind _widget (Default|AddQuesttoList (Variables|Default|GetMainWidget) (LocalVariables|GetLocalQuestActor)))
    (bind _output_get_2 (Variables|/Game/General_Blueprints/QuestSystem/QuestActors/MasterQuest_BP.MasterQuest_BP_C|SetQuestWidget (LocalVariables|GetLocalQuestActor) _widget))
    (Default|UpdateQuest _output_get_2)
    (if (or (LocalVariables|GetStart?) (<= (Utilities|Array|Length (Variables|Default|GetQuestActors)) 1))
      (CallFunction|SelectNewQuest (LocalVariables|GetLocalQuestActor) (Utilities|Array|Get(acopy) (Variables|/Game/UI_HUD_Blueprints/Quest_Widget.Quest_Widget_C|GetSubGoalWidget (Variables|/Game/General_Blueprints/QuestSystem/QuestActors/MasterQuest_BP.MasterQuest_BP_C|GetQuestWidget (LocalVariables|GetLocalQuestActor))))))
    (return true)
    (else
      (return false))))