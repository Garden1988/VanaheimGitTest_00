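; Base quest actor for the quest system that tracks which sub-goals of a quest are currently active.
; A list of active indices is seeded from the start indices and resolved against QuestInfo's SubGoals to rebuild CurrentGoals.
; Advancing replaces all active indices with the one after the highest, returning false when no sub-goal remains.
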(fn ConstructionScript)

(fn UpdateSubGoals
  (Utilities|Array|Clear (Variables|DonotTouch!|GetCurrentGoals))
  (for _array_element (Variables|DonotTouch!|GetCurrentGoal_Index)
    (Utilities|Array|Add (Variables|DonotTouch!|GetCurrentGoals) (Utilities|Array|Get(acopy) (.SubGoals (Utilities|Struct|BreakS_QuestInfo (Variables|UseMe!|GetQuestInfo))) _array_element)))
  (return))

(fn SetupStartGoals
  (Utilities|Array|Clear (Variables|DonotTouch!|GetCurrentGoal_Index))
  (Variables|DonotTouch!|SetCurrentGoal_Index (Variables|UseMe!|GetStartSubGoal_Index))
  (CallFunction|UpdateSubGoals)
  (return))

(fn GotoNextSubGoal
  (bind _currentgoal_index (Variables|DonotTouch!|GetCurrentGoal_Index))
  (bind _currentgoal_index_2 (Variables|DonotTouch!|GetCurrentGoal_Index))
  (bind _maxvalue (Math|Integer|MaxOfIntArray _currentgoal_index))
  (bind _returnvalue (+ _maxvalue 1))
  (if (<= _returnvalue (Utilities|Array|LastIndex (.SubGoals (Utilities|Struct|BreakS_QuestInfo (Variables|UseMe!|GetQuestInfo)))))
    (Variables|Default|SetNext%20Index _returnvalue)
    (Utilities|Array|Clear _currentgoal_index_2)
    (Utilities|Array|Add _currentgoal_index_2 (Variables|Default|GetNext%20Index))
    (CallFunction|UpdateSubGoals)
    (return true)
    (else
      (return false))))